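; Trap platform that falls after the player character steps into its trigger box, then respawns at its original spot.
; The first player overlap passes a DoOnce, waits a configurable delay, then enables physics simulation on the Cube so it drops.
; After a second delay it spawns a fresh instance of its own class at the transform saved on BeginPlay and destroys itself, which re-arms the trap.
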(event OnComponentBeginOverlap(Box)
  (params (OverlappedComponent :type Primitive%20Component%20Object%20Reference) (OtherActor :type Actor%20Object%20Reference) (OtherComp :type Primitive%20Component%20Object%20Reference) (OtherBodyIndex :type Integer) (bFromSweep :type Boolean) (SweepResult :type Hit%20Result%20Structure%20%28by%20ref%29))
  (if (== OtherActor (Game|GetPlayerCharacter 0))
    (Utilities|FlowControl|DoOnce false
      (:Completed
        (Utilities|FlowControl|Delay (Variables|Default|GetCoolddownBeforeFalling))
        (Physics|SetSimulatePhysics (Variables|Default|GetCube) true)
        (Utilities|FlowControl|Delay (Variables|Default|GetCoolddownBeforeRemovingActor))
        (CallFunction|RespawnPlatform)
        (Actor|DestroyActor)))))

(event Custom|RespawnPlatform
  (Game|SpawnActorfromClass "BP_FallingPlatform_C" (Variables|Default|GetBeginPlayTransform) "Undefined" 0 0))

(event EventBeginPlay
  (Variables|Default|SetBeginPlayTransform (Transformation|GetActorTransform)))

(fn ConstructionScript)