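; BP_PlayerMainMenu is the main menu player Blueprint that loads the saved time to beat and opens the menu on BeginPlay.
; It asynchronously loads the SaveTimer slot and copies its minutes and seconds into My_GameInstance, or saves a fresh BP_SaveTimer if none exists.
; Both paths then create WBP_MainMenu, show the mouse cursor and switch input to UI only.
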(event EventBeginPlay
  (bind _returnvalue (Game|GetPlayerController 0))
  (bind _asmy_game_instance (Utilities|Casting|CastToMy_GameInstance (Game|GetGameInstance)))
  (Variables|Default|SetGameInstanceRef _asmy_game_instance)
  (bind _returnvalue_2 (SaveGame|DoesSaveGameExist "SaveTimer"))
  (if _returnvalue_2
    (bind _savegame (|AsyncLoadGamefromSlot "SaveTimer")
      (:Completed
        (bind _asbp_save_timer (Utilities|Casting|CastToBP_SaveTimer _savegame))
        (Default|SetMinutestoBeat (Variables|Default|GetGameInstanceRef) (Variables|/Game/Blueprints/SaveGame/BP_SaveTimer.BP_SaveTimer_C|GetMinutes _asbp_save_timer))
        (Default|SetSecondstoBeat (Variables|Default|GetGameInstanceRef) (Variables|/Game/Blueprints/SaveGame/BP_SaveTimer.BP_SaveTimer_C|GetSeconds _asbp_save_timer))))
    (else
      (bind _returnvalue_3 (SaveGame|CreateSaveGameObject "/Game/Blueprints/SaveGame/BP_SaveTimer.BP_SaveTimer_C"))
      (SaveGame|SaveGametoSlot _returnvalue_3 "SaveTimer")))
  (bind _returnvalue_4 (UserInterface|CreateWidget "/Game/Blueprints/UI/WBP_MainMenu.WBP_MainMenu_C" (Game|GetPlayerController 0)))
  (Variables|Default|SetMainMenuRef _returnvalue_4)
  (UserInterface|Viewport|AddtoViewport _returnvalue_4 0)
  (Variables|/Script/Engine.PlayerController|SetbShowMouseCursor _returnvalue true)
  (Input|SetInputModeUIOnly _returnvalue _returnvalue_4 "DoNotLock"))

(fn ConstructionScript)